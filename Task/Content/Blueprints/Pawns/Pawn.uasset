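; Walking AI pawn that heads toward a Target and destroys itself with explosion effect and sound on arrival.
; Tick drives forward movement, re-aims at the Target when a sphere trace hits it, and turns randomly at obstacles or ledges found by line traces.
; With CanRespite or BackWalk set, timers alternate walking with pausing or backing up and periodically re-path to the Target.
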(event EventTick
  (params (DeltaSeconds :type Float%20%28single-precision%29))
  (if (not (Variables|Target|GetFinal))
    ;[1 1 1] Movement
    (Pawn|Input|AddMovementInput (Transformation|GetActorForwardVector) (Variables|Movement|GetAxisMove) false)
    (Target|CheckTarget)
    (Target|CheckObstacle)
    (Target|CheckFinal)))

(event EventBeginPlay
  ;[1 1 1] SetSpeed
  (Variables|/Script/Engine.CharacterMovementComponent|SetMaxWalkSpeed (Variables|Character|GetCharacterMovement) (Variables|Movement|Get%20Speed))
  ;[1 1 1] Recpite
  (if (or (Variables|Recpite|GetCanRespite) (Variables|Recpite|GetBackWalk))
    (bind _returnvalue (Utilities|Time|SetTimerbyFunctionName 0 "Recpite" 1.0))
    (Variables|Recpite|SetRecpiteTimer _returnvalue)
    (bind _returnvalue_2 (Utilities|Time|SetTimerbyFunctionName 0 "FindTarget" 1.5 true))
    (Variables|Target|SetFindTargetTimer _returnvalue_2)))

(fn ConstructionScript)

(fn Recpite
  (Variables|Movement|SetAxisMove (select (Variables|Recpite|GetBackWalk) -1.0 0.0))
  (bind _returnvalue (Utilities|Time|SetTimerbyFunctionName 0 "Walk" 0.5))
  (Variables|Recpite|SetWalkTimer _returnvalue))

(fn Walk
  (Variables|Movement|SetAxisMove 1.0)
  (bind _returnvalue (Utilities|Time|SetTimerbyFunctionName 0 "Recpite" 1.0))
  (Variables|Recpite|SetRecpiteTimer _returnvalue))

(fn FindTarget
  (Utilities|IsValid (Variables|Target|GetTarget)
    (:Is%20Valid
      (Transformation|SetActorRotation (Math|Rotator|MakeRotator 0.0 0.0 (.yaw (Math|Rotator|FindLookatRotation (Transformation|GetActorLocation) (Transformation|GetActorLocation (Variables|Target|GetTarget))))))
      (AI|Navigation|SimpleMovetoLocation (Pawn|GetController) (Transformation|GetActorLocation (Variables|Target|GetTarget))))))

(fn CheckTarget
  (Utilities|IsValid (Variables|Target|GetTarget)
    (:Is%20Valid
      (bind _outhit (Collision|SphereTraceByChannel (Transformation|GetActorLocation) (+ (Transformation|GetActorLocation (Variables|Target|GetTarget)) "0.000000,0.000000,15.000000") 15.0 "TraceTypeQuery1" false (Utilities|Array|MakeArray (Variables|Target|GetNest)) "None" true "(R=1.000000,G=0.000000,B=0.000000,A=1.000000)" "(R=0.000000,G=1.000000,B=0.000000,A=1.000000)" 0.0))
      (if (== (Variables|Target|GetTarget) (.HitActor (Collision|BreakHitResult _outhit)))
        (Target|FindTarget)))))

(fn CheckObstacle
  (bind _returnvalue (Transformation|GetActorLocation))
  (bind _returnvalue_2 (Transformation|GetActorForwardVector))
  (bind _returnvalue_3 (Transformation|GetActorLocation))
  (bind _checkobstacledist (Variables|Movement|GetCheckObstacleDist))
  (bind _checkobstacledist_2 (Variables|Movement|GetCheckObstacleDist))
  (bind _returnvalue_4 (* _returnvalue_2 (Math|Vector|MakeVector _checkobstacledist_2 _checkobstacledist_2 _checkobstacledist_2)))
  (bind _returnvalue_5 (+ _returnvalue _returnvalue_4))
  (bind _outhit (Collision|LineTraceByChannel _returnvalue_3 (+ _returnvalue_3 (* (Transformation|GetActorForwardVector) (Math|Vector|MakeVector _checkobstacledist _checkobstacledist _checkobstacledist))) "TraceTypeQuery1" false (Utilities|Array|MakeArray (Variables|Target|GetNest) (Variables|Target|GetTarget)) "None" true "(R=1.000000,G=0.000000,B=0.000000,A=1.000000)" "(R=0.000000,G=1.000000,B=0.000000,A=1.000000)" 0.0))
  (Utilities|IsValid (.HitActor (Collision|BreakHitResult _outhit))
    (:Is%20Valid
      (Class|Actor|AddActorWorldRotation (Math|Rotator|MakeRotator 0.0 0.0 (select (Math|Random|RandomBool) 1e+01 -1e+01)) :!label _label))
    (:Is%20Not%20Valid
      (bind _outhit_2 (Collision|LineTraceByChannel _returnvalue_5 (- _returnvalue_5 "0.000000,0.000000,250.000000") "TraceTypeQuery1" false (Utilities|Array|MakeArray (Variables|Target|GetNest) (Variables|Target|GetTarget)) "None" true "(R=1.000000,G=0.000000,B=0.000000,A=1.000000)" "(R=0.000000,G=1.000000,B=0.000000,A=1.000000)" 0.0))
      (if (not (Utilities|IsValid (.HitActor (Collision|BreakHitResult _outhit_2))))
        (goto _label)))))

(fn CheckFinal
  (bind _returnvalue (Transformation|GetActorLocation))
  (bind _target (Variables|Target|GetTarget))
  (bind _returnvalue_2 (Transformation|GetActorLocation _target))
  (if (Math|Boolean|ANDBoolean (Math|Float|InRange(Float) (.x _returnvalue) (- (.x _returnvalue_2) 1e+01) (+ (.x _returnvalue_2) 1e+01)) (Math|Float|InRange(Float) (.y _returnvalue) (- (.y _returnvalue_2) 1e+01) (+ (.y _returnvalue_2) 1e+01)) (Math|Float|InRange(Float) (.z _returnvalue) (- (.z _returnvalue_2) 5e+01) (+ (.z _returnvalue_2) 5e+01)))
    (Target|StopWalking)))

(fn StopWalking
  (Variables|Target|SetFinal true)
  (Utilities|Time|ClearandInvalidateTimerbyHandle (Variables|Target|GetFindTargetTimer))
  (Utilities|Time|ClearandInvalidateTimerbyHandle (Variables|Recpite|GetRecpiteTimer))
  (Utilities|Time|ClearandInvalidateTimerbyHandle (Variables|Recpite|GetWalkTimer))
  (Variables|Movement|SetAxisMove 0.0)
  (Effects|SpawnEmitteratLocation "/Game/Assets/Particles/P_Explosion2.P_Explosion2" (Transformation|GetActorLocation) "0, 0, 0" "2.000000,2.000000,2.000000")
  (Audio|SpawnSoundatLocation "/Game/Assets/Sounds/LaserShot_Cue.LaserShot_Cue" (Transformation|GetActorLocation) "0, 0, 0" 1.0 1.0 0.0 0 0)
  (Actor|DestroyActor))