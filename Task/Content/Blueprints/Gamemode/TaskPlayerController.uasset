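; TaskPlayerController is the player controller for the Task game mode that sets up the main UI when play begins.
; On BeginPlay it casts the current game mode to TaskGamemode and stores it, stopping if the cast fails.
; It then creates W_MainWidget with that game mode passed in, adds it to the viewport and switches input to UI-only, focused on the widget.
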(event EventBeginPlay
  ;[1 1 1] SetGamemode
  (bind _astask_gamemode (Utilities|Casting|CastToTaskGamemode (Game|GetGameMode)))
  (Variables|Gamemode|SetGamemode _astask_gamemode)
  (CallFunction|AddMainWidget))

(fn ConstructionScript)

(fn AddMainWidget
  (bind _returnvalue (UserInterface|CreateWidget "/Game/Blueprints/UI/MainWidget/W_MainWidget.W_MainWidget_C" self (Variables|Gamemode|GetGamemode)))
  (bind _output_get (Variables|Widget|SetW_MainWidget _returnvalue))
  (UserInterface|Viewport|AddtoViewport _output_get 0)
  (Input|SetInputModeUIOnly self (Variables|Widget|GetW_MainWidget) "DoNotLock" false))